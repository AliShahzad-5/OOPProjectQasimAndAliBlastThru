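; Player paddle pawn for a brick-breaker style game (BlastThru2).
; On BeginPlay it hides the cursor, adds the Enhanced Input mapping context and creates the player HUD.
; Move input slides the paddle along local Z by PaddleSpeed with sweep collision.
; Pause input opens the pause menu widget, switches to UI-only input with the cursor shown and pauses the game.
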(event Input|EnhancedActionEvents|EnhancedInputActionMove_IA
  (params (ActionValue :type Float%20%28double-precision%29) (ElapsedSeconds :type Float%20%28double-precision%29) (TriggeredSeconds :type Float%20%28double-precision%29) (InputAction :type Input%20Action%20Object%20Reference :default "/Game/Input/Move_IA.Move_IA"))
  (Transformation|AddLocalOffset (Variables|Default|GetPaddle) (Math|Vector|MakeVector 0.0 0.0 (* ActionValue (Variables|Default|GetPaddleSpeed))) true false))

(event Input|EnhancedActionEvents|EnhancedInputActionIA_Pause
  (params (ActionValue :type Boolean) (ElapsedSeconds :type Float%20%28double-precision%29) (TriggeredSeconds :type Float%20%28double-precision%29) (InputAction :type Input%20Action%20Object%20Reference :default "/Game/Input/IA_Pause.IA_Pause"))
  (bind _returnvalue (Game|GetPlayerController 0))
  (:Started
    (bind _returnvalue_2 (UserInterface|CreateWidget "/Game/Blueprints/PauseMenu_WB.PauseMenu_WB_C"))
    (UserInterface|Viewport|AddtoViewport _returnvalue_2 0)
    (Variables|/Script/Engine.PlayerController|SetbShowMouseCursor _returnvalue true)
    (Input|SetInputModeUIOnly _returnvalue 0 "DoNotLock" false)
    (Game|SetGamePaused true)))

(event EventBeginPlay
  (bind _returnvalue (Game|GetPlayerController 0))
  (Variables|/Script/Engine.PlayerController|SetbShowMouseCursor _returnvalue false)
  (Input|SetInputModeGameOnly _returnvalue false)
  (bind _asplayer_controller (Utilities|Casting|CastToPlayerController (Pawn|GetController)))
  (Utilities|IsValid (PlayerController|LocalPlayerSubsystems|GetEnhancedInputLocalPlayerSubsystem _asplayer_controller)
    (:Is%20Valid
      (Input|AddMappingContext (PlayerController|LocalPlayerSubsystems|GetEnhancedInputLocalPlayerSubsystem _asplayer_controller) "/Game/Input/BlastThru2_IMC.BlastThru2_IMC" 0 "(bIgnoreAllPressedKeysUntilRelease=True,bForceImmediately=False,bNotifyUserSettings=False)")
      (bind _returnvalue_2 (UserInterface|CreateWidget "/Game/Blueprints/Player_HUD.Player_HUD_C"))
      (bind _output_get (Variables|Default|SetPlayerHud _returnvalue_2))
      (UserInterface|Viewport|AddtoViewport _output_get 0))))

(event Collision|EventActorBeginOverlap
  (params (OtherActor :type Actor%20Object%20Reference)))

(event EventTick
  (params (DeltaSeconds :type Float%20%28single-precision%29)))

(fn ConstructionScript)