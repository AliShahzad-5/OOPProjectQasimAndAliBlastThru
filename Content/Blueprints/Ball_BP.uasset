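; Ball actor for a brick-breaker game, driven by physics on a sphere and launched with an impulse at BeginPlay.
; Each hit plays a beep, raises the speed by one and clamps velocity magnitude to that speed; brick hits update the score on the paddle pawn's HUD.
; On destruction, it asks the spawner for a new ball if the paddle has lives left, otherwise it shows the Game Over widget.
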(event EventBeginPlay
  (Physics|AddImpulse (Variables|Default|GetSphere) (Math|Vector|MakeVector -1e+03 0.0 0.0) "None" true)
  (bind _aspaddle_bp (Utilities|Casting|CastToPaddle_BP (Game|Player|GetPlayerPawn 0)))
  (Variables|Default|SetAs%20Paddle%20BP _aspaddle_bp))

(event Collision|EventActorBeginOverlap
  (params (OtherActor :type Actor%20Object%20Reference)))

(event EventTick
  (params (DeltaSeconds :type Float%20%28single-precision%29)))

(event Collision|EventHit
  (params (MyComp :type Primitive%20Component%20Object%20Reference) (Other :type Actor%20Object%20Reference) (OtherComp :type Primitive%20Component%20Object%20Reference) (bSelfMoved :type Boolean) (HitLocation :type Vector :default "0, 0, 0") (HitNormal :type Vector :default "0, 0, 0") (NormalImpulse :type Vector :default "0, 0, 0") (Hit :type Hit%20Result%20Structure%20%28by%20ref%29))
  (bind _sphere (Variables|Default|GetSphere))
  (Audio|PlaySoundatLocation "/Game/Music/ping_pong_8bit_beeep.ping_pong_8bit_beeep" (Transformation|GetActorLocation) "0, 0, 0" 1.0 1.0 0.0 0 0 0 0)
  (Variables|Default|SetBallSpeed (+ (Variables|Default|GetBallSpeed) 1.0))
  (bind _returnvalue (Physics|GetPhysicsLinearVelocity _sphere "None"))
  (Physics|SetPhysicsLinearVelocity _sphere (Math|Vector|ClampVectorSize _returnvalue (Variables|Default|GetBallSpeed) (Variables|Default|GetBallSpeed)) false "None")
  (if (Actor|ActorHasTag Other "Brick")
    (Default|UpdateScore (Variables|/Game/Blueprints/Paddle_BP.Paddle_BP_C|GetPlayerHud (Variables|Default|GetAs%20Paddle%20BP)))))

(event EventDestroyed
  (if (> (Variables|/Game/Blueprints/Paddle_BP.Paddle_BP_C|GetLives (Variables|Default|GetAs%20Paddle%20BP)) 0)
    (Default|SpawnBall (Variables|Default|GetBallSpawnerRef))
    (Utilities|FlowControl|Delay 1.0)
    (else
      (bind _returnvalue (UserInterface|CreateWidget "/Game/Blueprints/GameOver_WBP.GameOver_WBP_C"))
      (UserInterface|Viewport|AddtoViewport _returnvalue 0))))

(fn ConstructionScript)